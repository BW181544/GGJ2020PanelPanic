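; Camera point that positions a given camera to follow the player within bounds and also supplies a respawn location.
; SetCameraPos works in Deadzone box space, holding Y and Z centered while the player is inside, then offsetting by the overshoot, capped at the Limit-to-Deadzone extent difference.
; Depth and rotation come from the Scene component, applied directly without smoothing.
; BeginPlay caches the RespawnPoint world location, returned by GetRespawnPoint.
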(event EventBeginPlay
  (Variables|Default|SetRespawnLocation (Transformation|GetWorldLocation (Variables|Default|GetRespawnPoint))))

(event EventSetCameraPos
  (params (PlayerRef :type Character%20Object%20Reference) (CameraRef :type Camera%20Component%20Object%20Reference))
  (bind _returnvalue (Transformation|GetActorLocation PlayerRef))
  (bind _deadzone (Variables|Default|GetDeadzone))
  (bind _deadzone_2 (Variables|Default|GetDeadzone))
  (bind _limit (Variables|Default|GetLimit))
  (bind _returnvalue_2 (Components|Box|GetScaledBoxExtent _deadzone))
  (bind _returnvalue_3 (Transformation|GetWorldTransform _deadzone_2))
  (bind _returnvalue_4 (Components|Box|GetScaledBoxExtent _limit))
  (bind _returnvalue_5 (Math|Transform|InverseTransformLocation _returnvalue_3 _returnvalue))
  (bind _returnvalue_6 (- (.z _returnvalue_4) (.z _returnvalue_2)))
  (bind _returnvalue_7 (- (.y _returnvalue_4) (.y _returnvalue_2)))
  (bind _returnvalue_8 (Math|Float|Absolute(Float) (.y _returnvalue_5)))
  (bind _returnvalue_9 (Math|Float|Absolute(Float) (.z _returnvalue_5)))
  (bind _returnvalue_10 (Math|Float|Absolute(Float) _returnvalue_6))
  (bind _returnvalue_11 (Math|Float|Absolute(Float) _returnvalue_7))
  (bind _returnvalue_12 (- _returnvalue_8 (.y _returnvalue_2)))
  (bind _returnvalue_13 (- _returnvalue_9 (.z _returnvalue_2)))
  (bind _returnvalue_14 (Math|Float|Absolute(Float) _returnvalue_13))
  (bind _returnvalue_15 (Math|Float|Absolute(Float) _returnvalue_12))
  (bind _returnvalue_16 (Math|Float|Min(Float) _returnvalue_14 _returnvalue_10))
  (bind _returnvalue_17 (Math|Float|Min(Float) _returnvalue_15 _returnvalue_11))
  (Transformation|SetWorldLocationAndRotation CameraRef (Math|Transform|TransformLocation (Transformation|GetWorldTransform (Variables|Default|GetDeadzone)) (Math|Vector|MakeVector (.x (Math|Transform|InverseTransformLocation (Transformation|GetWorldTransform (Variables|Default|GetDeadzone)) (Transformation|GetWorldLocation (Variables|Default|GetScene)))) (select (> _returnvalue_8 (.y _returnvalue_2)) (select (< (.y _returnvalue_5) 0.0) (CallFunction|NegateF _returnvalue_17) _returnvalue_17) 0.0) (select (> _returnvalue_9 (.z _returnvalue_2)) (select (< (.z _returnvalue_5) 0.0) (CallFunction|NegateF _returnvalue_16) _returnvalue_16) 0.0))) (Transformation|GetWorldRotation (Variables|Default|GetScene)) false false))

(fn ConstructionScript)

(fn NegateF
  (params (In :type Float%20%28single-precision%29))
  (bind _result (Math|Float|NegateFloat In)
    (:%20%20
      (return _result))))

(fn GetRespawnPoint
  (return (Variables|Default|GetRespawnLocation)))