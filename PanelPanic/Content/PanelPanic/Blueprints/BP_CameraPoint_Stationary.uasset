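; Stationary camera point for Panel Panic that places a supplied camera at a fixed view and provides a respawn location.
; SetCameraPos snaps the camera to the Scene component's world location and rotation, using the player reference only in a validity check.
; The RespawnPoint component's world location is cached on BeginPlay and returned by GetRespawnPoint.
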(event EventBeginPlay
  (Variables|Default|SetRespawnLocation (Transformation|GetWorldLocation (Variables|Default|GetRespawnPoint))))

(event EventSetCameraPos
  (params (PlayerRef :type Character%20Object%20Reference) (CameraRef :type Camera%20Component%20Object%20Reference))
  (bind _scene (Variables|Default|GetScene))
  (bind _returnvalue (Transformation|GetWorldTransform _scene))
  (if (and (Utilities|IsValid PlayerRef) (Utilities|IsValid CameraRef))
    (Transformation|SetWorldLocationAndRotation CameraRef (.location _returnvalue) (.rotation _returnvalue) false false)))

(fn ConstructionScript)

(fn GetRespawnPoint
  (return (Variables|Default|GetRespawnLocation)))