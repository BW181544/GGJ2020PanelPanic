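; Trigger volume that moves the overlapping BP_Character's camera to a referenced camera point.
; Begin overlap calls TransitionToCameraPoint, and end overlap reports that camera point back to the character through ReportEndOverlap.
; When IsDirectional is set, it transitions only if the character's local-space position lies on the volume's positive X side at entry.
; The construction script shows the Arrow component only for directional volumes.
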(event OnComponentBeginOverlap(Volume)
  (params (OverlappedComponent :type Primitive%20Component%20Object%20Reference) (OtherActor :type Actor%20Object%20Reference) (OtherComp :type Primitive%20Component%20Object%20Reference) (OtherBodyIndex :type Integer) (bFromSweep :type Boolean) (SweepResult :type Hit%20Result%20Structure%20%28by%20ref%29))
  (bind _asbp_character (Utilities|Casting|CastToBP_Character OtherActor))
  (if (Variables|Default|GetIsDirectional)
    (if (Math|Float|NearlyEqual(Float) (Math|Vector|DotProduct (Math|Vector|Normalize (Math|Vector|MakeVector (.x (- (Math|Transform|InverseTransformLocation (Transformation|GetWorldTransform (Variables|Default|GetScene)) (Transformation|GetActorLocation _asbp_character)) "0, 0, 0")) 0.0 0.0)) "1.000000, 0, 0") 1.0 0.1)
      (Default|TransitiontoCameraPoint _asbp_character (Variables|Default|GetCameraPointRef) :!label _label))
    (else
      (goto _label))))

(event OnComponentEndOverlap(Volume)
  (params (OverlappedComponent :type Primitive%20Component%20Object%20Reference) (OtherActor :type Actor%20Object%20Reference) (OtherComp :type Primitive%20Component%20Object%20Reference) (OtherBodyIndex :type Integer))
  (bind _asbp_character (Utilities|Casting|CastToBP_Character OtherActor))
  (Default|ReportEndOverlap _asbp_character (Variables|Default|GetCameraPointRef)))

(fn ConstructionScript
  (Rendering|SetVisibility (Variables|Default|GetArrow) (Variables|Default|GetIsDirectional) false))