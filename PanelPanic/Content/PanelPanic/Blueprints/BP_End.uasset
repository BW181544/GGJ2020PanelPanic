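; End-of-game trigger that hands the player over to a closing camera sequence when BP_Character overlaps its box, disabling player input.
; TransitionToPoint blends the passed-in camera to the CameraPath spline start and the actor's rotation, returning true on arrival.
; SetCameraPos advances the camera along the spline over TravelDuration, then calls FinishedGame on the character.
; Both camera steps rely on external calls supplying DeltaTime, and GetRespawnPoint only returns zero.
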(event OnComponentBeginOverlap(Box)
  (params (OverlappedComponent :type Primitive%20Component%20Object%20Reference) (OtherActor :type Actor%20Object%20Reference) (OtherComp :type Primitive%20Component%20Object%20Reference) (OtherBodyIndex :type Integer) (bFromSweep :type Boolean) (SweepResult :type Hit%20Result%20Structure%20%28by%20ref%29))
  (bind _asbp_character (Utilities|Casting|CastToBP_Character OtherActor))
  (Default|TransitiontoCameraPoint _asbp_character self)
  (Input|DisableInput (Game|GetPlayerController 0)))

(event EventSetCameraPos
  (params (PlayerRef :type Character%20Object%20Reference) (CameraRef :type Camera%20Component%20Object%20Reference) (DeltaTime :type Float%20%28single-precision%29))
  (if (and (Utilities|IsValid PlayerRef) (Utilities|IsValid CameraRef))
    (bind _output_get (Variables|Default|SetTotalTravelTime (Math|Float|Clamp(Float) (+ (Variables|Default|GetTotalTravelTime) DeltaTime) 0.0 (Variables|Default|GetTravelDuration))))
    (Transformation|SetWorldLocation CameraRef (Spline|GetLocationatDistanceAlongSpline (Variables|Default|GetCameraPath) (* (/ _output_get (Variables|Default|GetTravelDuration)) (Variables|Default|GetPathLength)) "World") false false)
    (if (== (Variables|Default|GetTotalTravelTime) (Variables|Default|GetTravelDuration))
      (bind _asbp_character (Utilities|Casting|CastToBP_Character PlayerRef))
      (Default|FinishedGame _asbp_character))))

(event EventBeginPlay
  (Variables|Default|SetPathLength (Spline|GetSplineLength (Variables|Default|GetCameraPath))))

(fn ConstructionScript)

(fn GetRespawnPoint
  (return "0, 0, 0"))

(fn TransitiontoPoint
  (params (DeltaTime :type Float%20%28single-precision%29) (PlayerRef :type BP%20Character%20Object%20Reference) (CameraRef :type Camera%20Component%20Object%20Reference) (OldCameraTransform :type Transform))
  (bind _returnvalue (Transformation|GetActorRotation))
  (bind _camerapath (Variables|Default|GetCameraPath))
  (bind _returnvalue_2 (Spline|GetLocationatSplinePoint _camerapath 0 "World"))
  (bind _output_get (Variables|Default|SetTotalTime (Math|Float|Min(Float) (+ (Variables|Default|GetTotalTime) DeltaTime) (Variables|Default|GetTransitionTime))))
  (Transformation|SetWorldLocationAndRotation CameraRef (Math|Vector|Lerp(Vector) (.location OldCameraTransform) _returnvalue_2 (/ _output_get (Variables|Default|GetTransitionTime))) (Math|Rotator|Lerp(Rotator) (.rotation OldCameraTransform) _returnvalue (/ _output_get (Variables|Default|GetTransitionTime)) true) false false)
  (if (and (Math|Vector|Equal(Vector) (Math|Vector|Lerp(Vector) (.location OldCameraTransform) _returnvalue_2 (/ _output_get (Variables|Default|GetTransitionTime))) _returnvalue_2 0.0001) (Math|Rotator|Equal(Rotator) (Math|Rotator|Lerp(Rotator) (.rotation OldCameraTransform) _returnvalue (/ _output_get (Variables|Default|GetTransitionTime)) true) _returnvalue 0.0001))
    (Variables|Default|SetTotalTime 0.0)
    (return true)
    (else
      (return false))))