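; BP_MovingSprite is an actor whose Paper2D sprite travels along a spline when a BP_Character enters its trigger box.
; The spline length is cached on BeginPlay, and StartMove plays the Movement timeline, whose Alpha scales that length into a distance along the path.
; Each update places the sprite at that world location without sweeping, and completion calls the MoveFinished dispatcher.
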(event OnComponentBeginOverlap(Box)
  (params (OverlappedComponent :type Primitive%20Component%20Object%20Reference) (OtherActor :type Actor%20Object%20Reference) (OtherComp :type Primitive%20Component%20Object%20Reference) (OtherBodyIndex :type Integer) (bFromSweep :type Boolean) (SweepResult :type Hit%20Result%20Structure%20%28by%20ref%29))
  (Utilities|Casting|CastToBP_Character OtherActor)
  (CallFunction|StartMove))

(event Custom|StartMove
  (bind _alpha (Timeline|Movement Play)
    (:Update
      (Transformation|SetWorldLocation (Variables|Default|GetPaperSprite) (Spline|GetLocationatDistanceAlongSpline (Variables|Default|GetSpline) (* _alpha (Variables|Default|GetPathLength)) "World") false false))
    (:Finished
      (Default|CallMoveFinished))))

(event EventBeginPlay
  (Variables|Default|SetPathLength (Spline|GetSplineLength (Variables|Default|GetSpline))))

(fn ConstructionScript)