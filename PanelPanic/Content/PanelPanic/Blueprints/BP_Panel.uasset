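; BP_Panel is a Panel Panic panel that fits four sprite edges around its box component.
; ResizePanelEdges calls SetPanelEdges, which runs SetEdge per side; the construction script's SetPanelEdges call is disconnected.
; SetEdge assigns the sprite, prints a debug scale readout, then positions and stretches the edge in the XZ plane.
; It derives both from box extent, EdgeThickness and sprite bounds divided by current scale.
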(event Custom|Resize%20Panel%20Edges
  (CallFunction|SetPanelEdges))

(event Custom|SetPanelEdges
  (CallFunction|SetEdge (Variables|Default|GetTop) (Variables|Default|GetTopEdge) "NewEnumerator0")
  (CallFunction|SetEdge (Variables|Default|GetBottom) (Variables|Default|GetBottomEdge) "NewEnumerator1")
  (CallFunction|SetEdge (Variables|Default|GetLeft) (Variables|Default|GetLeftEdge) "NewEnumerator2")
  (CallFunction|SetEdge (Variables|Default|GetRight) (Variables|Default|GetRightEdge) "NewEnumerator3"))

(fn ConstructionScript)

(fn SetEdge
  (params (Edge :type Paper%20Sprite%20Component%20Object%20Reference) (Sprite :type Paper%20Sprite%20Object%20Reference) (EdgeType :type PanelEdge%20Enum :default "NewEnumerator0"))
  (bind _boxextent (Collision|GetComponentBounds Edge))
  (bind _relativescale3d (Variables|/Script/Engine.SceneComponent|GetRelativeScale3D Edge))
  (bind _panel (Variables|Default|GetPanel))
  (bind _edgethickness (Variables|Default|GetEdgeThickness))
  (bind _returnvalue (/ (.x _boxextent) (.x _relativescale3d)))
  (bind _returnvalue_2 (/ (.z _boxextent) (.z _relativescale3d)))
  (bind _returnvalue_3 (/ (.x _boxextent) (.x _relativescale3d)))
  (bind _returnvalue_4 (/ (.z _boxextent) (.z _relativescale3d)))
  (bind _returnvalue_5 (Components|Box|GetScaledBoxExtent _panel))
  (bind _returnvalue_6 (/ (.z _returnvalue_5) _returnvalue_2))
  (bind _returnvalue_7 (/ (.x _returnvalue_5) _returnvalue))
  (bind _returnvalue_8 (* _returnvalue_4 _edgethickness))
  (bind _returnvalue_9 (* _returnvalue_3 _edgethickness))
  (bind _returnvalue_10 (- (.x _returnvalue_5) _returnvalue_9))
  (bind _returnvalue_11 (- (.z _returnvalue_5) _returnvalue_8))
  (LocalVariables|SetEdgeT EdgeType)
  (Rendering|Components|Sprite|SetSprite Edge Sprite)
  (Development|PrintText (Utilities|Text|FormatText "{Plane} / {Sprite}" (Utilities|Text|ToText(Float) (.x _relativescale3d) "HalfToEven") (Utilities|Text|ToText(Float) (.z _relativescale3d) "HalfToEven")))
  (Transformation|SetRelativeLocation Edge (+ (Variables|/Script/Engine.SceneComponent|GetRelativeLocation (Variables|Default|GetPanel)) (Utilities|Select :Index (LocalVariables|GetEdgeT) :NewEnumerator0 (Math|Vector|MakeVector 0.0 0.0 (Utilities|Select :Index (LocalVariables|GetEdgeT) :NewEnumerator0 (Utilities|Select :Index (LocalVariables|GetEdgeT) :NewEnumerator0 _returnvalue_11 :NewEnumerator1 _returnvalue_11 :NewEnumerator2 _returnvalue_10 :NewEnumerator3 _returnvalue_10) :NewEnumerator1 (* (Utilities|Select :Index (LocalVariables|GetEdgeT) :NewEnumerator0 _returnvalue_11 :NewEnumerator1 _returnvalue_11 :NewEnumerator2 _returnvalue_10 :NewEnumerator3 _returnvalue_10) -1.0) :NewEnumerator2 (Utilities|Select :Index (LocalVariables|GetEdgeT) :NewEnumerator0 _returnvalue_11 :NewEnumerator1 _returnvalue_11 :NewEnumerator2 _returnvalue_10 :NewEnumerator3 _returnvalue_10) :NewEnumerator3 (* (Utilities|Select :Index (LocalVariables|GetEdgeT) :NewEnumerator0 _returnvalue_11 :NewEnumerator1 _returnvalue_11 :NewEnumerator2 _returnvalue_10 :NewEnumerator3 _returnvalue_10) -1.0))) :NewEnumerator1 (Math|Vector|MakeVector 0.0 0.0 (Utilities|Select :Index (LocalVariables|GetEdgeT) :NewEnumerator0 (Utilities|Select :Index (LocalVariables|GetEdgeT) :NewEnumerator0 _returnvalue_11 :NewEnumerator1 _returnvalue_11 :NewEnumerator2 _returnvalue_10 :NewEnumerator3 _returnvalue_10) :NewEnumerator1 (* (Utilities|Select :Index (LocalVariables|GetEdgeT) :NewEnumerator0 _returnvalue_11 :NewEnumerator1 _returnvalue_11 :NewEnumerator2 _returnvalue_10 :NewEnumerator3 _returnvalue_10) -1.0) :NewEnumerator2 (Utilities|Select :Index (LocalVariables|GetEdgeT) :NewEnumerator0 _returnvalue_11 :NewEnumerator1 _returnvalue_11 :NewEnumerator2 _returnvalue_10 :NewEnumerator3 _returnvalue_10) :NewEnumerator3 (* (Utilities|Select :Index (LocalVariables|GetEdgeT) :NewEnumerator0 _returnvalue_11 :NewEnumerator1 _returnvalue_11 :NewEnumerator2 _returnvalue_10 :NewEnumerator3 _returnvalue_10) -1.0))) :NewEnumerator2 (Math|Vector|MakeVector (Utilities|Select :Index (LocalVariables|GetEdgeT) :NewEnumerator0 (Utilities|Select :Index (LocalVariables|GetEdgeT) :NewEnumerator0 _returnvalue_11 :NewEnumerator1 _returnvalue_11 :NewEnumerator2 _returnvalue_10 :NewEnumerator3 _returnvalue_10) :NewEnumerator1 (* (Utilities|Select :Index (LocalVariables|GetEdgeT) :NewEnumerator0 _returnvalue_11 :NewEnumerator1 _returnvalue_11 :NewEnumerator2 _returnvalue_10 :NewEnumerator3 _returnvalue_10) -1.0) :NewEnumerator2 (Utilities|Select :Index (LocalVariables|GetEdgeT) :NewEnumerator0 _returnvalue_11 :NewEnumerator1 _returnvalue_11 :NewEnumerator2 _returnvalue_10 :NewEnumerator3 _returnvalue_10) :NewEnumerator3 (* (Utilities|Select :Index (LocalVariables|GetEdgeT) :NewEnumerator0 _returnvalue_11 :NewEnumerator1 _returnvalue_11 :NewEnumerator2 _returnvalue_10 :NewEnumerator3 _returnvalue_10) -1.0)) 0.0 0.0) :NewEnumerator3 (Math|Vector|MakeVector (Utilities|Select :Index (LocalVariables|GetEdgeT) :NewEnumerator0 (Utilities|Select :Index (LocalVariables|GetEdgeT) :NewEnumerator0 _returnvalue_11 :NewEnumerator1 _returnvalue_11 :NewEnumerator2 _returnvalue_10 :NewEnumerator3 _returnvalue_10) :NewEnumerator1 (* (Utilities|Select :Index (LocalVariables|GetEdgeT) :NewEnumerator0 _returnvalue_11 :NewEnumerator1 _returnvalue_11 :NewEnumerator2 _returnvalue_10 :NewEnumerator3 _returnvalue_10) -1.0) :NewEnumerator2 (Utilities|Select :Index (LocalVariables|GetEdgeT) :NewEnumerator0 _returnvalue_11 :NewEnumerator1 _returnvalue_11 :NewEnumerator2 _returnvalue_10 :NewEnumerator3 _returnvalue_10) :NewEnumerator3 (* (Utilities|Select :Index (LocalVariables|GetEdgeT) :NewEnumerator0 _returnvalue_11 :NewEnumerator1 _returnvalue_11 :NewEnumerator2 _returnvalue_10 :NewEnumerator3 _returnvalue_10) -1.0)) 0.0 0.0))) false false)
  (Transformation|SetRelativeScale3D Edge (Utilities|Select :Index (LocalVariables|GetEdgeT) :NewEnumerator0 (Math|Vector|MakeVector (Utilities|Select :Index (LocalVariables|GetEdgeT) :NewEnumerator0 _returnvalue_7 :NewEnumerator1 _returnvalue_7 :NewEnumerator2 _returnvalue_6 :NewEnumerator3 _returnvalue_6) (.y (Variables|/Script/Engine.SceneComponent|GetRelativeScale3D Edge)) (Variables|Default|GetEdgeThickness)) :NewEnumerator1 (Math|Vector|MakeVector (Utilities|Select :Index (LocalVariables|GetEdgeT) :NewEnumerator0 _returnvalue_7 :NewEnumerator1 _returnvalue_7 :NewEnumerator2 _returnvalue_6 :NewEnumerator3 _returnvalue_6) (.y (Variables|/Script/Engine.SceneComponent|GetRelativeScale3D Edge)) (Variables|Default|GetEdgeThickness)) :NewEnumerator2 (Math|Vector|MakeVector (Variables|Default|GetEdgeThickness) (.y (Variables|/Script/Engine.SceneComponent|GetRelativeScale3D Edge)) (Utilities|Select :Index (LocalVariables|GetEdgeT) :NewEnumerator0 _returnvalue_7 :NewEnumerator1 _returnvalue_7 :NewEnumerator2 _returnvalue_6 :NewEnumerator3 _returnvalue_6)) :NewEnumerator3 (Math|Vector|MakeVector (Variables|Default|GetEdgeThickness) (.y (Variables|/Script/Engine.SceneComponent|GetRelativeScale3D Edge)) (Utilities|Select :Index (LocalVariables|GetEdgeT) :NewEnumerator0 _returnvalue_7 :NewEnumerator1 _returnvalue_7 :NewEnumerator2 _returnvalue_6 :NewEnumerator3 _returnvalue_6)))))