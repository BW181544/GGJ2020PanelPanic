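; Moving platform actor for Panel Panic that loops through a two-leg path relative to its spawn location, fading out on the second leg.
; Tick accumulates time and lerps the actor along cumulative offsets, each leg with its own duration.
; A dynamic material's Opacity drops during the second leg, then resets as the loop restarts from the origin instead of travelling back.
; The fade value is also printed every tick of that leg.
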(event EventTick
  (params (DeltaSeconds :type Float%20%28single-precision%29))
  (bind _defaultpos (Variables|Default|GetDefaultPos))
  (bind _pos1 (Variables|Default|Getpos1))
  (bind _defaultpos_2 (Variables|Default|GetDefaultPos))
  (bind _returnvalue (+ _defaultpos _pos1))
  (Variables|Default|SetTime (+ DeltaSeconds (Variables|Default|GetTime)))
  (switch int (Variables|Default|GetCurrentPos)
    (:0
      (Transformation|SetActorLocation (Math|Vector|Lerp(Vector) _defaultpos_2 (+ _defaultpos_2 (Variables|Default|Getpos1)) (/ (Variables|Default|GetTime) (Variables|Default|GetTimeFirstPos))) false false)
      (if (> (Variables|Default|GetTime) (Variables|Default|GetTimeFirstPos))
        (Variables|Default|SetTime 0.0)
        (Variables|Default|SetCurrentPos 1)))
    (:1
      (Transformation|SetActorLocation (Math|Vector|Lerp(Vector) _returnvalue (+ _returnvalue (Variables|Default|GetPos2)) (/ (Variables|Default|GetTime) (Variables|Default|GetTimeSecondPos))) false false)
      (Development|PrintString (Utilities|String|ToString(Float) (- 1.0 (/ (Variables|Default|GetTime) (Variables|Default|GetTimeSecondPos)))))
      (Rendering|Material|SetScalarParameterValue (Variables|Default|GetMID) "Opacity" (- 1.0 (/ (Variables|Default|GetTime) (Variables|Default|GetTimeSecondPos))) :!class /Script/Engine.MaterialInstanceDynamic)
      (if (> (Variables|Default|GetTime) (Variables|Default|GetTimeSecondPos))
        (Variables|Default|SetTime 0.0)
        (Variables|Default|SetCurrentPos 0)
        (Rendering|Material|SetScalarParameterValue (Variables|Default|GetMID) "Opacity" 1.0 :!class /Script/Engine.MaterialInstanceDynamic)))))

(event EventBeginPlay
  (bind _eer (Variables|Default|Geteer))
  (Variables|Default|SetDefaultPos (Transformation|GetActorLocation))
  (bind _returnvalue (Rendering|Material|CreateDynamicMaterialInstance _eer 0 (Rendering|Material|GetMaterial _eer 0) "None" :!class /Script/Engine.PrimitiveComponent))
  (Variables|Default|SetMID _returnvalue))

(fn ConstructionScript)